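; Game mode Blueprint for an Asteroids game that manages the start, HUD and game over screens.
; On BeginPlay it shows a start widget whose button starts the game and removes that widget.
; InitUI creates the HUD and binds to game state lives and score events, forwarding updates to it.
; Game over swaps the HUD for a game over widget showing the player's final score.
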(event `self.ReceiveBeginPlay`
  (`parent.ReceiveBeginPlay`)
  (bind _returnvalue (`|CreateWidget` "/Game/Asteroids/UIs/WBP_StartGame.WBP_StartGame_C"))
  (bind _output_get (set `self.StartGameWidget` _returnvalue))
  (`UserWidget.AddToViewport` _output_get 0)
  (add `Button.OnClicked` (`/Game/Asteroids/UIs/WBP_StartGame.StartButton` _output_get) (delegate `OnClicked_Event`)))

(event `OnClicked_Event`
  (`self.StartGame`)
  (`Widget.RemoveFromParent` (`self.StartGameWidget`)))

(event `self.InitUI`
  (bind _asteroidsgamestate (`self.asteroidsGameState`))
  (bind _returnvalue (`|CreateWidget` "/Game/Asteroids/UIs/WBP_Hud.WBP_Hud_C"))
  (bind _output_get (set `self.HudWidget` _returnvalue))
  (`UserWidget.AddToViewport` _output_get 0)
  (add `AsteroidsGameState.OnLivesUpdated` _asteroidsgamestate (delegate `self.UpdateLives`))
  (add `AsteroidsGameState.OnScoreUpdated` _asteroidsgamestate (delegate `self.UpdateScore`)))

(event `self.UpdateLives`
  (params (lives :type Integer))
  (`parent.UpdateLives` lives)
  (`/Game/Asteroids/UIs/WBP_Hud.LivesUpdated` (`self.HudWidget`) lives))

(event `self.UpdateScore`
  (params (score :type Integer))
  (`parent.UpdateScore` score)
  (`/Game/Asteroids/UIs/WBP_Hud.ScoreUpdated` (`self.HudWidget`) score))

(event `self.CallGameOverUI`
  (`Widget.RemoveFromParent` (`self.HudWidget`))
  (bind _returnvalue (`|CreateWidget` "/Game/Asteroids/UIs/WBP_GameOver.WBP_GameOver_C"))
  (bind _output_get (set `self.GameOverWidget` _returnvalue))
  (`UserWidget.AddToViewport` _output_get 0)
  (`/Game/Asteroids/UIs/WBP_GameOver.SetScore` _output_get (`AsteroidsGameState.GetPlayerScore` (`self.asteroidsGameState`))))

(fn `UserConstructionScript`)