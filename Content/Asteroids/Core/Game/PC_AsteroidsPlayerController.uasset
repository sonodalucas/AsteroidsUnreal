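; Player controller for the Asteroids game that creates and manages the HUD, start screen and game over UI.
; On BeginPlay it adds the HUD and start widget to the viewport.
; The start button is bound by authority: the server starts the match through GM_AsteroidsGameMode and closes the menu, while remote clients only close it.
; A CallGameOverUI event shows the game over widget with the passed score.
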(event `self.ReceiveBeginPlay`
  (`parent.ReceiveBeginPlay`)
  (`self.CreateHUD`)
  (`self.CreateStartGame`))

(event `CreateHUD`
  (bind _returnvalue (`|CreateWidget` "/Game/Asteroids/UIs/WBP_HUD.WBP_HUD_C" self))
  (bind _output_get (set `self.HudWidget` _returnvalue))
  (`UserWidget.AddToViewport` _output_get 0))

(event `OnClicked_Event`
  (`self.StartGame`)
  (`Widget.RemoveFromParent` (`self.startWidget`)))

(event `CreateStartGame`
  (bind _returnvalue (`|CreateWidget` "/Game/Asteroids/UIs/WBP_StartGame.WBP_StartGame_C" self))
  (bind _output_get (set `self.startWidget` _returnvalue))
  (`UserWidget.AddToViewport` _output_get 0)
  (`/Engine/EditorBlueprintResources/ActorMacros.Switch Has Authority`
    (:`Authority`
      (bind _startbutton (`/Game/Asteroids/UIs/WBP_StartGame.StartButton` _returnvalue))
      (add `Button.OnClicked` _startbutton (delegate `OnClicked_Event`)))
    (:`Remote`
      (add `Button.OnClicked` _startbutton (delegate `CustomEvent`)))))

(event `StartGame`
  (`AsteroidsGameMode.StartGame` (cast `/Game/Asteroids/Core/Game/GM_AsteroidsGameMode` (`GameplayStatics.GetGameMode`) :!pure true)))

(event `CustomEvent`
  (`Widget.RemoveFromParent` (`self.startWidget`)))

(event `CallGameOverUI`
  (params (Score :type Integer))
  (bind _returnvalue (`|CreateWidget` "/Game/Asteroids/UIs/WBP_GameOver.WBP_GameOver_C" self))
  (`UserWidget.AddToViewport` _returnvalue 0)
  (`/Game/Asteroids/UIs/WBP_GameOver.SetScore` _returnvalue Score))

(fn `UserConstructionScript`)