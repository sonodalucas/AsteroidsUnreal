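; Player ship for an Asteroids game, with a flipbook sprite that switches between thrust and idle.
; Enhanced Input drives thrust, turning, cooldown-limited shooting and hyperspace, each gated by the player controller's input lock.
; Turning goes through ServerRotateActor, and hits apply damage to the other actor.
; A timed invincibility flicker toggles sprite visibility with capsule collision disabled, then restores both.
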(event `self.ReceiveBeginPlay`
  (bind _aspc_asteroids_player_controller (cast `/Game/Asteroids/Core/Game/PC_AsteroidsPlayerController` (`self.GetController`)))
  (set `self.PlayerController` _aspc_asteroids_player_controller)
  (bind _returnvalue (pcsubsystem `EnhancedInputLocalPlayerSubsystem` _aspc_asteroids_player_controller))
  (`/Engine/EditorBlueprintResources/StandardMacros.IsValid` _returnvalue
    (:`Is Valid`
      (`EnhancedInputSubsystemInterface.AddMappingContext` _returnvalue "/Game/Asteroids/Input/IMC_Default.IMC_Default" 0 (struct)))))

(event `self.StartSpriteFlicker`
  (`PrimitiveComponent.SetCollisionEnabled` (`self.CapsuleComponent`) "NoCollision")
  (bind _returnvalue (`KismetSystemLibrary.K2_SetTimerDelegate` (delegate `ToggleVisibility`) (`self.FlickerDelay`) true))
  (`KismetSystemLibrary.Delay` (`self.invincibilityTime`))
  (`KismetSystemLibrary.K2_ClearAndInvalidateTimerHandle` _returnvalue)
  (`SceneComponent.SetVisibility` (`self.Sprite`) true false)
  (set `self.isInvincible` false)
  (`PrimitiveComponent.SetCollisionEnabled` (`self.CapsuleComponent`) "QueryOnly"))

(event `ToggleVisibility`
  (bind _sprite (`self.Sprite`))
  (`SceneComponent.SetVisibility` _sprite (not (`SceneComponent.bVisible` _sprite)) false))

(event `EnhancedInput|/Game/Asteroids/Input/Actions/IA_Shoot`
  (params (ActionValue :type Boolean) (ElapsedSeconds :type "Float (double-precision)") (TriggeredSeconds :type "Float (double-precision)") (InputAction :type "InputAction Object Reference" :default "/Game/Asteroids/Input/Actions/IA_Shoot.IA_Shoot"))
  (bind (_returnvalue_location _returnvalue_rotation) (`KismetMathLibrary.BreakTransform` (`SceneComponent.K2_GetComponentToWorld` (`self.BulletSpawnPosition`))))
  ;[0.1667 0.4879 1] Inputs
  (:`Triggered`
    (bind _returnvalue (`AsteroidsPlayerController.IsInputLocked` (`self.PlayerController`)))
    (if _returnvalue
      _
      (elif (`self.CanShoot`)
        (`self.ShootProjectile` _returnvalue_location _returnvalue_rotation true)
        (bind _returnvalue_2 (`AsteroidsPlayerController.IsInputLocked` (`self.PlayerController`)))
        (if (not _returnvalue_2)
          (set `self.CanShoot` false)
          (`KismetSystemLibrary.K2_SetTimerDelegate` (delegate `ReleaseShootLock`) (`self.ShootCooldown`)))))))

(event `self.ReceiveHit`
  (params (MyComp :type "PrimitiveComponent Object Reference") (Other :type "Actor Object Reference") (OtherComp :type "PrimitiveComponent Object Reference") (bSelfMoved :type Boolean) (HitLocation :type "Vector Structure") (HitNormal :type "Vector Structure") (NormalImpulse :type "Vector Structure") (Hit :type "HitResult Structure (by ref)"))
  (`GameplayStatics.ApplyDamage` Other 1.0 (`self.GetController`) self))

(event `ReleaseShootLock`
  ;[0.1667 0.4879 1] Inputs
  (set `self.CanShoot` true))

(event `EnhancedInput|/Game/Asteroids/Input/Actions/IA_Thrust`
  (params (ActionValue :type Boolean) (ElapsedSeconds :type "Float (double-precision)") (TriggeredSeconds :type "Float (double-precision)") (InputAction :type "InputAction Object Reference" :default "/Game/Asteroids/Input/Actions/IA_Thrust.IA_Thrust"))
  ;[0.1667 0.4879 1] Inputs
  (:`Triggered`
    (bind _returnvalue (`AsteroidsPlayerController.IsInputLocked` (`self.PlayerController`)))
    (if (not _returnvalue)
      (`self.AddMovementInput` (`self.GetActorForwardVector`))
      (`self.ChangeFlipbook` (`self.ThrustFlipbook`))))
  (:`Completed`
    (`self.ChangeFlipbook` (`self.IdleFlipbook`))))

(event `EnhancedInput|/Game/Asteroids/Input/Actions/IA_Turn`
  (params (ActionValue :type "Float (double-precision)") (ElapsedSeconds :type "Float (double-precision)") (TriggeredSeconds :type "Float (double-precision)") (InputAction :type "InputAction Object Reference" :default "/Game/Asteroids/Input/Actions/IA_Turn.IA_Turn"))
  ;[0.1667 0.4879 1] Inputs
  (:`Triggered`
    (bind _returnvalue (`AsteroidsPlayerController.IsInputLocked` (`self.PlayerController`)))
    (if (not _returnvalue)
      (`self.Server_RotateActor` (`KismetMathLibrary.MakeRotator` 0.0 (* ActionValue -1.0 (`self.turnVelocity`)))))))

(event `ChangeFlipbook`
  (params (NewFlipbook :type "PaperFlipbook Object Reference"))
  (`PaperFlipbookComponent.SetFlipbook` (`self.Sprite`) NewFlipbook))

(event `EnhancedInput|/Game/Asteroids/Input/Actions/IA_HyperSpace`
  (params (ActionValue :type Boolean) (ElapsedSeconds :type "Float (double-precision)") (TriggeredSeconds :type "Float (double-precision)") (InputAction :type "InputAction Object Reference" :default "/Game/Asteroids/Input/Actions/IA_HyperSpace.IA_HyperSpace"))
  ;[0.1667 0.4879 1] Inputs
  (:`Triggered`
    (bind _returnvalue (`AsteroidsPlayerController.IsInputLocked` (`self.PlayerController`)))
    (if (not _returnvalue)
      (`self.ActivateHyperSpace`))))

(fn `UserConstructionScript`)